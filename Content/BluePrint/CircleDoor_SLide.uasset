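; Sliding door actor that opens once enough switches have been activated.
; ActivateSwitchFuction increments a counter on each call and triggers OpenDoor when the count reaches or exceeds RequiredSwitch.
; OpenDoor plays the TL_Opendoor timeline, whose alpha lerps the static mesh along its relative X axis to the open position.
; The file contains no closing or counter reset logic.
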(event `OpenDoor`
  (bind (_direction _alpha) (`Timeline|TL_Opendoor`)
    (:`Update`
      (`SceneComponent.K2_SetRelativeLocation` (`self.StaticMesh`) (`KismetMathLibrary.MakeVector` (`KismetMathLibrary.Lerp` 0.0 500.0 _alpha)) false false))))

(fn `ActivateSwitchFuction`
  (set `self.ActivateSwitch` (+ (`self.ActivateSwitch`) 1))
  (if (>= (`self.ActivateSwitch`) (`self.RequiredSwitch`))
    (`self.OpenDoor`)))

(fn `UserConstructionScript`)