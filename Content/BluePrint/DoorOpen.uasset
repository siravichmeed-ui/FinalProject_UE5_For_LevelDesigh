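; DoorOpen is an interactable double door that swings open and closed on IA_Interact.
; A DoorRotation timeline pitches DoorL and DoorR in opposite directions, playing when closed and reversing otherwise.
; Tick derives the DoorClose flag from the timeline's current value.
; The Box trigger enables player input on both begin and end overlap, so leaving the box does not disable interaction.
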(event `EnhancedInput|/Game/Input/Actions/IA_Interact`
  (params (ActionValue :type "Vector2D Structure") (ElapsedSeconds :type "Float (double-precision)") (TriggeredSeconds :type "Float (double-precision)") (InputAction :type "InputAction Object Reference" :default "/Game/Input/Actions/IA_Interact.IA_Interact"))
  (:`Triggered`
    (if (`self.DoorClose`)
      (bind (_direction _door) (`Timeline|DoorRotation` :!label _label)
        (:`Update`
          (bind _returnvalue (`KismetMathLibrary.MakeRotator` 0.0 _door))
          (`SceneComponent.K2_SetRelativeLocationAndRotation` (`self.Door L`) (0.0 0.0 1.0) _returnvalue false false)
          (`SceneComponent.K2_SetRelativeLocationAndRotation` (`self.Door R`) (0.0 0.0 1.0) (* _returnvalue -1.0) false false)))
      (else
        (goto _label :!via `Reverse`)))))

(event `self.ReceiveTick`
  (params (DeltaSeconds :type "Float (single-precision)"))
  (set `self.DoorClose` (< (stale `EnhancedInput|/Game/Input/Actions/IA_Interact` _door) 1.0)))

(event `self.Box.OnComponentBeginOverlap`
  (params (OverlappedComponent :type "PrimitiveComponent Object Reference") (OtherActor :type "Actor Object Reference") (OtherComp :type "PrimitiveComponent Object Reference") (OtherBodyIndex :type Integer) (bFromSweep :type Boolean) (SweepResult :type "HitResult Structure (by ref)"))
  (`self.EnableInput` (`GameplayStatics.GetPlayerController` 0)))

(event `self.Box.OnComponentEndOverlap`
  (params (OverlappedComponent :type "PrimitiveComponent Object Reference") (OtherActor :type "Actor Object Reference") (OtherComp :type "PrimitiveComponent Object Reference") (OtherBodyIndex :type Integer))
  (`self.EnableInput` (`GameplayStatics.GetPlayerController` 0)))

(fn `UserConstructionScript`)