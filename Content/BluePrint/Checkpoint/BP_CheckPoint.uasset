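; BP_CheckPoint is a checkpoint actor that registers itself as the active checkpoint when the player reaches it.
; When the player character overlaps its Box, it switches the Cylinder material to blue and prints a debug message.
; It then stores a reference to itself in the CheckPoint variable of BP_ThirdPersonGameMode.
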(event `Change To Blue`
  (`PrimitiveComponent.SetMaterial` (`self.Cylinder`) 0 "/Game/BluePrint/Checkpoint/Blue.Blue"))

(event `self.Box.OnComponentBeginOverlap`
  (params (OverlappedComponent :type "PrimitiveComponent Object Reference") (OtherActor :type "Actor Object Reference") (OtherComp :type "PrimitiveComponent Object Reference") (OtherBodyIndex :type Integer) (bFromSweep :type Boolean) (SweepResult :type "HitResult Structure (by ref)"))
  (if (== OtherActor (`GameplayStatics.GetPlayerCharacter` 0))
    (`self.Change To Blue`)
    (`KismetSystemLibrary.PrintString` "Checkpoint")
    (bind _asbp_third_person_game_mode (cast `/Game/ThirdPerson/Blueprints/BP_ThirdPersonGameMode` (`GameplayStatics.GetGameMode`)))
    (set `/Game/ThirdPerson/Blueprints/BP_ThirdPersonGameMode.CheckPoint` self _asbp_third_person_game_mode)))

(fn `UserConstructionScript`)